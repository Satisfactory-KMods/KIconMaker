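; Editor-placed capture rig that renders item or building classes to PNG icons, named from the cleaned class name.
; Construction and update events apply the class to a child actor, set arm, FOV and light, and force LOD 0.
; Optional coloring writes primary and secondary colors into custom primitive data.
; Export writes the render target directly, or first redraws it through an invert-alpha material when FixAlpha is set.
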(event `ForceUpdate`
  (`self.Func Update Camera Manuell`)
  ;[1 1 1] New Stuff
  (bind _returnvalue (`KismetMaterialLibrary.CreateDynamicMaterialInstance` "/KIconMaker/M_RT_InvertAlpha.M_RT_InvertAlpha"))
  (set `self.ExportMaterial` _returnvalue))

(event `ImportName`
  (`self.ImpName`))

(event `ResetAll`
  (set `self.mItemClass` null)
  (set `self.mBuildingClass` null)
  (set `self.mItemMesh` null))

(event `UpdateCamera`
  (`self.Func Update Camera Manuell`))

(event `Export`
  (`self.ImportName`)
  (`self.ExportIcon`))

(event `ExportIcon`
  (if (`self.FixAlpha`)
    ;[1 1 1] New Stuff
    (`|ExecutionSequence`
      (:`then_0`
        (`KismetRenderingLibrary.ClearRenderTarget2D` (`self.ExportTarget`) (struct)))
      (:`then_1`
        (`KismetRenderingLibrary.DrawMaterialToRenderTarget` (`self.ExportTarget`) (`self.ExportMaterial`)))
      (:`then_2`
        (`KismetRenderingLibrary.ExportRenderTarget` (`self.ExportTarget`) (`self.mExportPath`) (`KismetStringLibrary.Concat_StrStr` "Icon_" (`self.mName`) ".png"))))
    (else
      (`KismetRenderingLibrary.ExportRenderTarget` "/KIconMaker/RT_Custom.RT_Custom" (`self.mExportPath`) (`KismetStringLibrary.Concat_StrStr` "Icon_" (`self.mName`) ".png")))))

(fn `Func Update Camera Manuell`
  (locals (Preview :type "CameraComponent Object Reference"))
  (bind _mitemclass (`self.mItemClass`))
  (bind (_msecondarycolor_r _msecondarycolor_g _msecondarycolor_b) (break `LinearColor` (`self.mSecondaryColor`)))
  (bind (_mprimarycolor_r _mprimarycolor_g _mprimarycolor_b) (break `LinearColor` (`self.mPrimaryColor`)))
  (set `local.Preview` (`self.mWindowPreview`))
  (if (`KismetSystemLibrary.IsValidClass` _mitemclass)
    (`/KIconMaker/Capture/BP_CaptureActor.setClass` (`self.CaptureActor`) _mitemclass)
    (elif (`KismetSystemLibrary.IsValidClass` (`self.mBuildingClass`))
      (`/KIconMaker/Capture/BP_CaptureActor.setClass` (`self.CaptureActor`) (`self.mBuildingClass`))))
  (`|ExecutionSequence`
    (:`then_0`
      (set `SpringArmComponent.TargetArmLength` (`self.mCameraArm`) (`self.mArm`))
      (`SceneComponent.K2_SetRelativeRotation` (`self.mArm`) (`self.mCameraRotation`) false false)
      (bind _output_get (set `SceneCaptureComponent2D.FOVAngle` (`self.mFOVAngle`) (`self.mExportCapture`)))
      (`CameraComponent.SetFieldOfView` (`local.Preview`) _output_get)
      (`SceneComponent.K2_SetRelativeLocation` (`self.mArm`) (`self.mCameraLocation`) false false)
      (`CameraComponent.SetAspectRatio` (`local.Preview`) 1.0))
    (:`then_1`
      (`self.UpdateLight`))
    (:`then_2`
      (`/Engine/EditorBlueprintResources/StandardMacros.IsValid` null
        (:`Is Valid`
          (for _array_element (`self.K2_GetComponentsByClass` "/Script/FactoryGame.FGColoredInstanceMeshProxy")
            (`StaticMeshComponent.SetForcedLodModel` _array_element 0)
            (`PrimitiveComponent.SetCullDistance` _array_element 4999999913984.0)))))
    (:`then_3`
      (if (`self.mUseColoring`)
        (for _array_element_2 (`self.K2_GetComponentsByClass` "/Script/Engine.PrimitiveComponent")
          (for (_array_element_3 _array_index) (`|MakeArray` _mprimarycolor_r _mprimarycolor_g _mprimarycolor_b _msecondarycolor_r _msecondarycolor_g _msecondarycolor_b 0.0 0.0 0.0 0.0 0.0 0.0 0.0 0.0 0.0 0.0 0.0 0.0 0.0 0.0 0.0 :!type "Float (double-precision)")
            (`PrimitiveComponent.SetCustomPrimitiveDataFloat` _array_element_2 _array_index _array_element_3)))))))

(fn `GetName`
  (returns (Name :type Text))
  (bind _mitemclass (`self.mItemClass`))
  (bind _mbuildingclass (`self.mBuildingClass`))
  (return (select `bool` (`KismetSystemLibrary.IsValidClass` _mitemclass) :`false` (select `bool` (`KismetSystemLibrary.IsValidClass` _mbuildingclass) :`false` "Icon" :`true` (`KismetTextLibrary.Conv_StringToText` (`KismetStringLibrary.Replace` (`KismetStringLibrary.Replace` (`KismetStringLibrary.Replace` (`KismetStringLibrary.Replace` (`KismetStringLibrary.Replace` (`KismetSystemLibrary.GetClassDisplayName` _mbuildingclass) "SlugDesc_") "EggDesc_") "_C") "Desc_") "Build_"))) :`true` (`KismetTextLibrary.Conv_StringToText` (`KismetStringLibrary.Replace` (`KismetStringLibrary.Replace` (`KismetStringLibrary.Replace` (`KismetStringLibrary.Replace` (`KismetSystemLibrary.GetClassDisplayName` _mitemclass) "SlugDesc_") "EggDesc_") "_C") "Desc_")))))

(fn `ImpName`
  (if (or (`KismetSystemLibrary.IsValidClass` (`self.mBuildingClass`)) (`KismetSystemLibrary.IsValidClass` (`self.mItemClass`)))
    (set `self.mName` (`KismetStringLibrary.Replace` (`KismetStringLibrary.Replace` (`KismetTextLibrary.Conv_TextToString` (`self.GetName`)) " " "_") "#"))))

(fn `UpdateLight`
  (bind _lightcomponent (`Light.LightComponent` (`self.mLight`)))
  (`LightComponent.SetIntensity` _lightcomponent (`self.mLightIntensity`))
  (`SceneComponent.K2_SetWorldRotation` _lightcomponent (`KismetMathLibrary.SelectRotator` (`KismetMathLibrary.FindLookAtRotation` (`SceneComponent.K2_GetComponentLocation` (`self.mWindowPreview`)) (`SceneComponent.K2_GetComponentLocation` (`self.mArm`))) (`self.mSkyRotation`) (`self.mUseCameraToActorRotation`)) false false))

(fn `UserConstructionScript`
  (`self.Func Update Camera Manuell`)
  ;[1 1 1] New Stuff
  (bind _returnvalue (`KismetMaterialLibrary.CreateDynamicMaterialInstance` "/KIconMaker/M_RT_InvertAlpha.M_RT_InvertAlpha"))
  (set `self.ExportMaterial` _returnvalue)
  (`parent.UserConstructionScript`))