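; BP_CaptureActor spawns a preview mesh for a given class, apparently as the subject of a capture.
; Its setClass event destroys the previously spawned actor, then stores the new class.
; For an FGItemDescriptor class it spawns a StaticMeshActor at the world origin, applies the item's mesh and keeps it for later removal.
; FGBuildable classes are cast-checked but nothing is spawned for them.
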(event `setClass`
  (params (Class :type "Object Class Reference"))
  (bind _old (`self.old`))
  (`|ExecutionSequence`
    (:`then_0`
      (`/Engine/EditorBlueprintResources/StandardMacros.IsValid` _old
        (:`Is Valid`
          (`self.K2_DestroyActor` _old))))
    (:`then_1`
      (bind _output_get (set `self.Class` Class))
      (bind _asfgitem_descriptor (castclass `FGItemDescriptor` _output_get)
        (:`then`
          (bind _returnvalue (`|SpawnActorFromClass` "/Script/Engine.StaticMeshActor" (`KismetMathLibrary.MakeTransform` (0.0 0.0 0.0)) "Undefined" "OverrideRootScale" null null))
          (`StaticMeshComponent.SetStaticMesh` (`StaticMeshActor.StaticMeshComponent` _returnvalue) (`FGItemDescriptor.GetItemMesh` _asfgitem_descriptor))
          (set `self.old` _returnvalue))
        (:`CastFailed`
          (castclass `FGBuildable` _output_get))))))

(fn `UserConstructionScript`)